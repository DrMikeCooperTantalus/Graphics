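; Actor component that fades its owner's skeletal mesh toward invisibility and back, toggled by the P debug key.
; BeginPlay caches the original materials and creates dynamic instances from FXMaterials, leaving the originals applied.
; Tick moves the current alpha linearly toward the target over BlendDuration and passes it to SetAlpha.
; SetAlpha drives each instance's Alpha parameter, swapping material sets only when alpha crosses zero, so originals render when fully visible.
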(event EventBeginPlay
  ;[0.15 0.15 0.15 0.5] Set up Dynamic material instances so we can tweak their alpha later
  (bind _output_get (Variables|Default|SetSkeletalMesh (Actor|GetComponentbyClass (Components|GetOwner) "/Script/Engine.SkeletalMeshComponent")))
  (for (_array_element _array_index) (Variables|Default|GetFXMaterials)
    (Utilities|Array|Add (Variables|Default|GetOriginalMaterials) (Rendering|Material|GetMaterial _output_get _array_index))
    (bind _returnvalue (Rendering|Material|CreateDynamicMaterialInstance _output_get _array_index _array_element "None" :!class /Script/Engine.PrimitiveComponent))
    (Utilities|Array|Add (Variables|Default|GetDynamicMaterials) _returnvalue)
    (Rendering|Material|SetMaterial (Variables|Default|GetSkeletalMesh) _array_index (Utilities|Array|Get(acopy) (Variables|Default|GetOriginalMaterials) _array_index))))

(event EventTick
  (params (DeltaSeconds :type Float%20%28single-precision%29))
  (bind _targetalpha (Variables|Default|GetTargetAlpha))
  (bind _targetalpha_2 (Variables|Default|GetTargetAlpha))
  (Utilities|FlowControl|Sequence
    (:then_0
      (if (> (Variables|Default|GetTargetAlpha) (Variables|Default|GetCurrentAlpha))
        ;[0.15 0.15 0.15 0.5] Becoming invisible, counting up to a TargetAlpha of 1
        (Variables|Default|SetCurrentAlpha (+ (Variables|Default|GetCurrentAlpha) (/ DeltaSeconds (Variables|Default|GetBlendDuration))))
        (if (> (Variables|Default|GetCurrentAlpha) _targetalpha_2)
          (Variables|Default|SetCurrentAlpha _targetalpha_2))
        (else
          ;[0.15 0.15 0.15 0.5] Becoming visible again, counting down to TargetAlpha of 0
          (if (< (Variables|Default|GetTargetAlpha) (Variables|Default|GetCurrentAlpha))
            (Variables|Default|SetCurrentAlpha (- (Variables|Default|GetCurrentAlpha) (/ DeltaSeconds (Variables|Default|GetBlendDuration))))
            (if (< (Variables|Default|GetCurrentAlpha) _targetalpha)
              (Variables|Default|SetCurrentAlpha _targetalpha))))))
    (:then_1
      (CallFunction|SetAlpha (Variables|Default|GetCurrentAlpha)))))

(event Input|KeyboardEvents|DebugKeyP
  (params (Key :type Key%20Structure :default "None") (ActionValue :type Input%20Action%20Value%20Structure))
  (:Pressed
    (Variables|Default|SetTargetAlpha (- 1.0 (Variables|Default|GetTargetAlpha)))))

(fn SetAlpha
  (params (A :type Float%20%28double-precision%29))
  ;[0.15 0.15 0.15 0.5] Update Alpha values on dynamic materials
  (bind _output_get (Variables|Default|SetCurrentAlpha A))
  (for _array_element (Variables|Default|GetDynamicMaterials)
    (Rendering|Material|SetScalarParameterValue _array_element "Alpha" _output_get :!class /Script/Engine.MaterialInstanceDynamic))
  ;[0.15 0.15 0.15 0.5] Check if we should use the original materials (alpha == 0) or the dynamic blend ones and switch if we've changed that requirement.
  (if (!= (Variables|Default|GetUsingDynamicMaterials) (> (Variables|Default|GetCurrentAlpha) 0.0))
    (bind _output_get_2 (Variables|Default|SetUsingDynamicMaterials (> (Variables|Default|GetCurrentAlpha) 0.0)))
    (if _output_get_2
      (CallFunction|SetMaterials (Variables|Default|GetDynamicMaterials))
      (else
        (CallFunction|SetMaterials (Variables|Default|GetOriginalMaterials))))))

(fn SetMaterials
  (params (Materials :type Array%20of%20Material%20Interface%20Object%20References))
  (for (_ _array_index) Materials
    (Rendering|Material|SetMaterial (Variables|Default|GetSkeletalMesh) _array_index (Utilities|Array|Get(acopy) Materials _array_index))))